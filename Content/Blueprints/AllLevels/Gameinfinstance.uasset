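; Game instance that manages menu flow and multiplayer sessions, opening the main menu, or options on first run, based on a save check.
; Show events create UI widgets, most cached, though the loading screen's first call skips the viewport.
; Host settings create a session that opens Lobby as a listen server; other events join or destroy sessions.
; Failures, network and travel errors route to an error-display macro, empty here like both string converters.
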(event `SaveGameCheck`
  ;[1 1 1] Verificar juego guardado
  (bind _returnvalue (`GameplayStatics.DoesSaveGameExist` (`self.PlayerSettingsSave`)))
  (if _returnvalue
    (`self.ShowMainMenu`)
    (set `self.CreatedSaveFile?` true)
    (else
      (`self.ShowOptionsMenu`) ; Se configura para ver el Cursor del mause
      (set `PlayerController.bShowMouseCursor` true (`GameplayStatics.GetPlayerController` 0)))))

(event `ShowMainMenu`
  (bind _returnvalue (`GameplayStatics.GetPlayerController` 0))
  ;[1 1 1] Mostrar el menu principal y activar el cursor del mause
  (`/Engine/EditorBlueprintResources/StandardMacros.IsValid` (`self.MainMenuWB`) ; El widget is valid?  --- Se esta solicitando un jugador propietario
    (:`Is Valid`
      _)
    (:`Is Not Valid`
      (bind _returnvalue_2 (`|CreateWidget` "/Game/UI/MainMenu/MainMenu.MainMenu_C" _returnvalue)) ; Llamar class MainMenu
      (set `self.MainMenuWB` _returnvalue_2) ; Es valido para agreagar la ventana garafica
    ))
  (`UserWidget.AddToViewport` (`self.MainMenuWB`) 0) ; --- Se esta solicitando un jugador propietario
  (set `PlayerController.bShowMouseCursor` true _returnvalue) ; Cursosr de mause
)

(event `ShowLoadingScreen`
  ;[1 1 1] Muestra la pantalla de carga cuando se la llama
  (`/Engine/EditorBlueprintResources/StandardMacros.IsValid` (`self.LoadingScreenWB`)
    (:`Is Valid`
      (`UserWidget.AddToViewport` (`self.LoadingScreenWB`) 0))
    (:`Is Not Valid`
      (bind _returnvalue (`|CreateWidget` "/Game/UI/AllLevels/LoadingScreen.LoadingScreen_C" (`GameplayStatics.GetPlayerController` 0)))
      (set `self.LoadingScreenWB` _returnvalue))))

(event `LaunchLobby`
  (params (NumberOfPlayers :type Integer) (EnableLan :type Boolean) (ServerName :type Text))
  ;[1 1 1] Iniciar el Lobby con la configuracion del host
  (set `self.MaxPlayers` NumberOfPlayers)
  (set `self.ServerName` ServerName)
  (`self.ShowLoadingScreen`)
  (`CreateSessionCallbackProxy.CreateSession` (`GameplayStatics.GetPlayerController` 0) (`self.MaxPlayers`) EnableLan ; Las conexiones publicas provendran del servidor que lop definio
    (:`OnSuccess`
      (`GameplayStatics.OpenLevel` "Lobby" true "Listen"))
    (:`OnFailure`
      (`self.DisplayErrorMenssage` "Failed to create session. Please try Again ") ; Macro
    )))

(event `ShowHostMenu`
  ;[1 1 1] Host Game Menu  (El host define las carateristicas del servidor)
  (`/Engine/EditorBlueprintResources/StandardMacros.IsValid` (`self.HostMenuWB`)
    (:`Is Valid`
      _)
    (:`Is Not Valid`
      (bind _returnvalue (`|CreateWidget` "/Game/UI/MainMenu/HostMenu.HostMenu_C" (`GameplayStatics.GetPlayerController` 0))) ; Se agrega al widget el menu del host
      (set `self.HostMenuWB` _returnvalue)))
  (`UserWidget.AddToViewport` (`self.HostMenuWB`) 0))

(event `ShowServerMenu`
  ;[1 1 1] Mostrar Menu del servidor : creado cada vez que se llama
  (bind _returnvalue (`|CreateWidget` "/Game/UI/MainMenu/ServerMenu.ServerMenu_C" (`GameplayStatics.GetPlayerController` 0)))
  (`UserWidget.AddToViewport` _returnvalue 0))

(event `JoinServer`
  (params (SessionToJoin :type "BlueprintSessionResult Structure"))
  ;[1 1 1] Unirse a un servidor - llamado desde el Menu Servidor
  (`self.ShowLoadingScreen`) ; Llamar pantalla de carga
  (`JoinSessionCallbackProxy.JoinSession` (`GameplayStatics.GetPlayerController` 0) SessionToJoin
    (:`OnFailure`
      (`self.DisplayErrorMenssage` "Failed to join session. Please try Again ") ; Macro
    )))

(event `ShowOptionsMenu`
  ;[1 1 1] Mostrar la opccion del Menu
  (`/Engine/EditorBlueprintResources/StandardMacros.IsValid` (`self.OptionsMenuWB`)
    (:`Is Valid`
      _)
    (:`Is Not Valid`
      (bind _returnvalue (`|CreateWidget` "/Game/UI/MainMenu/OptionsMenu.OptionsMenu_C"))
      (set `self.OptionsMenuWB` _returnvalue)))
  (`UserWidget.AddToViewport` (`self.OptionsMenuWB`) 0)
  (if (not (`self.CreatedSaveFile?`))
    (set `/Game/UI/MainMenu/OptionsMenu.WelcomeMessageVis` "Visible" (`self.OptionsMenuWB`))))

(event `self.HandleNetworkError`
  (params (FailureType :type "ENetworkFailure Enum" :default "NetDriverAlreadyExists") (bIsServer :type Boolean))
  ;[1 1 1] Manejar errores de red y mostrar mensaje
  (if bIsServer
    _
    (else
      _))
  (`self.DisplayErrorMenssage` (`self.NetErrorToString` FailureType)))

(event `self.HandleTravelError`
  (params (FailureType :type "ETravelFailure Enum" :default "NoLevel"))
  ;[1 1 1] Manejar los errores de viaje y mostrar el mensaje
  (`self.DisplayErrorMenssage` (`self.TravelErrorToString` FailureType)))

(event `DestroySessionCaller`
  (params (PlayerController :type "PlayerController Object Reference"))
  ;[1 1 1] Destruir sesion cuando sea llamado
  (`DestroySessionCallbackProxy.DestroySession` PlayerController))

(fn `NetErrorToString`
  (params (FailureType :type "ENetworkFailure Enum" :default "NetDriverAlreadyExists"))
  (returns (OutString :type String))
  (return ""))

(fn `TravelErrorToString`
  (params (FailureType :type "ETravelFailure Enum" :default "NoLevel"))
  (returns (OutString :type String))
  (return ""))